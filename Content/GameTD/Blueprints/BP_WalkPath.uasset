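; BP_WalkPath is a walk path for the GameTD game, defined by an array of path node actors.
; Its GetNextPathNode function takes an index and returns the world location of that node.
; An index past the end of the array falls back to the last node's location, with no guard for an empty array.
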(fn `Get Next Path Node`
  (params (Index :type Integer))
  (returns (ReturnValue :type "Vector Structure"))
  (bind _pathnodearray (`self.PathNodeArray`))
  (bind _index (`local.Index`))
  (bind _returnvalue (`KismetArrayLibrary.Array_Length` _pathnodearray))
  (if (< _index _returnvalue)
    (return (`Actor.K2_GetActorLocation` (`|GetArrayItem` _pathnodearray _index)))
    (else
      (return (`Actor.K2_GetActorLocation` (`|GetArrayItem` _pathnodearray (- _returnvalue 1)))))))