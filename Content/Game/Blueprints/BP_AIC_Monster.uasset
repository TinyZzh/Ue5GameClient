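; AI controller for the monster that runs the BT_Monster behavior tree on BeginPlay and tracks the player by sight.
; Its perception component forwards target updates to HandleSightSense, which ignores non-sight stimuli and any actor other than the first player's character.
; That function feeds the Blackboard, setting TargetActor while the player is seen, or clearing it and storing LastKnownLocation when sight is lost.
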(event `self.ReceiveBeginPlay`
  (`self.RunBehaviorTree` "/Game/Game/Blueprints/BT_Monster.BT_Monster"))

(event `self.AI感知组件.OnTargetPerceptionUpdated`
  (params (Actor :type "Actor Object Reference") (Stimulus :type "AIStimulus Structure"))
  (`self.HandleSightSense` Actor Stimulus))

(fn `HandleSightSense`
  (params (Actor :type "Actor Object Reference") (Stimulus :type "AIStimulus Structure"))
  (bind _returnvalue (`GameplayStatics.GetPlayerCharacter` 0))
  (bind (_stimulus_age _stimulus_expirationage _stimulus_strength _stimulus_stimuluslocation _stimulus_receiverlocation _stimulus_tag _stimulus_bsuccessfullysensed) (break `AIStimulus` (`local.Stimulus`)))
  (bind _blackboard (`self.Blackboard`))
  (bind _returnvalue_2 (`AIPerceptionSystem.GetSenseClassForStimulus` Stimulus))
  (if (== _returnvalue_2 "/Script/AIModule.AISense_Sight")
    (if (== Actor _returnvalue)
      (`BlackboardComponent.SetValueAsObject` _blackboard "TargetActor" (`KismetMathLibrary.SelectObject` _returnvalue null _stimulus_bsuccessfullysensed))
      (if (not _stimulus_bsuccessfullysensed)
        (`BlackboardComponent.SetValueAsVector` _blackboard "LastKnownLocation" _stimulus_stimuluslocation))
      (else
        (return)))
    (else
      (return))))

(fn `UserConstructionScript`)