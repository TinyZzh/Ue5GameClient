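; BP_Door is an interactable door that the top-down character swings open and closed with the F key while nearby.
; Box overlap enables and disables input and opens and closes a Gate, printing a message when the character cast fails.
; F release passes the Gate into a FlipFlop that alternately plays and reverses a timeline, mapping its value to the Door's relative yaw.
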(event `Key|F`
  (params (Key :type "Key Structure"))
  (:`Released`
    (`/Engine/EditorBlueprintResources/StandardMacros.Gate` true :!label _label
      (:`Exit`
        (`/Engine/EditorBlueprintResources/StandardMacros.FlipFlop`
          (:`A`
            (bind (_direction _doorrotationz) (`Timeline|旋转` :!label _label_2)
              (:`Update`
                (`SceneComponent.K2_SetRelativeRotation` (`self.Door`) (`KismetMathLibrary.MakeRotator` 0.0 0.0 (`KismetMathLibrary.MapRangeClamped` _doorrotationz 0.0 1.0 0.0 90.0)) false false))))
          (:`B`
            (goto _label_2 :!via `Reverse`)))))))

(event `self.Box.OnComponentBeginOverlap`
  (params (OverlappedComponent :type "PrimitiveComponent Object Reference") (OtherActor :type "Actor Object Reference") (OtherComp :type "PrimitiveComponent Object Reference") (OtherBodyIndex :type Integer) (bFromSweep :type Boolean) (SweepResult :type "HitResult Structure (by ref)"))
  (cast `/Game/TopDown/Blueprints/BP_TopDownCharacter` OtherActor
    (:`then`
      (`self.EnableInput` (`GameplayStatics.GetPlayerController` 0)) ; 进入区域才激活按键输入
      (goto _label :!via `Open`))
    (:`CastFailed`
      (`KismetSystemLibrary.PrintText` "转换Character失败" :!label _label_3))))

(event `self.Box.OnComponentEndOverlap`
  (params (OverlappedComponent :type "PrimitiveComponent Object Reference") (OtherActor :type "Actor Object Reference") (OtherComp :type "PrimitiveComponent Object Reference") (OtherBodyIndex :type Integer))
  (cast `/Game/TopDown/Blueprints/BP_TopDownCharacter` OtherActor
    (:`then`
      (`self.DisableInput` (`GameplayStatics.GetPlayerController` 0)) ; 禁用按键输入
      (goto _label :!via `Close`))
    (:`CastFailed`
      (goto _label_3))))

(fn `UserConstructionScript`)